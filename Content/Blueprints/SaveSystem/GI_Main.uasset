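; GI_Main is a Game Instance that loads and persists the player's audio volume settings through a Save_Audio save game.
; On Init it loads the settings slot if one exists, otherwise it creates a new save object in memory.
; SFX and BGM volume events update that cached object and write it straight back to the slot, printing a message on success.
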(event Custom|LoadSetting
  (bind _returnvalue (SaveGame|DoesSaveGameExist (Variables|Default|GetSettingsSlot)))
  (if _returnvalue
    (bind _returnvalue_2 (SaveGame|LoadGamefromSlot (Variables|Default|GetSettingsSlot)))
    (bind _assave_audio (Utilities|Casting|CastToSave_Audio _returnvalue_2))
    (Variables|Default|SetSGB_Settings _assave_audio)
    (else
      (bind _returnvalue_3 (SaveGame|CreateSaveGameObject "/Game/Blueprints/SaveSystem/Save_Audio.Save_Audio_C"))
      (Variables|Default|SetSGB_Settings _returnvalue_3))))

(event Custom|SaveSettings
  (bind _returnvalue (SaveGame|SaveGametoSlot (Variables|Default|GetSGB_Settings) (Variables|Default|GetSettingsSlot)))
  (if _returnvalue
    (Development|PrintString "Saved")))

(event Custom|SaveVolumeSFX
  (params (VolumeSFX :type Float%20%28double-precision%29))
  (Variables|/Game/Blueprints/SaveSystem/Save_Audio.Save_Audio_C|SetVolumeSFX (Variables|Default|GetSGB_Settings) VolumeSFX)
  (CallFunction|SaveSettings))

(event Custom|SaveVolumeBGM
  (params (VolumeBGM :type Float%20%28double-precision%29))
  (Variables|/Game/Blueprints/SaveSystem/Save_Audio.Save_Audio_C|SetVolumeBGM (Variables|Default|GetSGB_Settings) VolumeBGM)
  (CallFunction|SaveSettings))

(event EventInit
  (CallFunction|LoadSetting))