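; BP_Tengu is the Tengu enemy character Blueprint, adding hit feedback on top of its parent class.
; On BeginPlay it binds to the HealthComponent's damage-taken event.
; Each hit plays the LongNeckHit sound and spawns an enlarged Niagara magic hit effect at the actor's location.
; Tick, overlap and construction add no logic of their own.
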(event Custom|OnHealthDamageTaken_Event
  (params (HealthComponent :type Health%20Component%20Object%20Reference) (Damage :type Integer) (CurrentHealth :type Integer) (DamageCauser :type Actor%20Object%20Reference) (DamageInstigator :type Controller%20Object%20Reference))
  (Utilities|FlowControl|Sequence
    (:then_0
      (Audio|PlaySoundatLocation "/Game/Assets/Audio/SFX/SFX_LongNeckHit_Cue.SFX_LongNeckHit_Cue" (Transformation|GetActorLocation) "0, 0, 0" 1.0 1.0 0.0 0 0 0 0))
    (:then_1
      (Niagara|SpawnSystematLocation "/Game/Free_Magic/VFX_Niagara/NS_Free_Magic_HitEnemy.NS_Free_Magic_HitEnemy" (Transformation|GetActorLocation) "0, 0, 0" "5.000000,5.000000,5.000000" true true "None" false))))

(event EventBeginPlay
  (|CallParentFunction)
  (EventDispatchers|AssignOnHealthDamageTaken (Variables|Default|GetHealthComponent) (delegate Custom|OnHealthDamageTaken_Event)))

(event Collision|EventActorBeginOverlap
  (params (OtherActor :type Actor%20Object%20Reference))
  (|CallParentFunction OtherActor) ; This node is disabled and will not be called.\nDrag off pins to build functionality.
)

(event EventTick
  (params (DeltaSeconds :type Float%20%28single-precision%29))
  (|CallParentFunction DeltaSeconds) ; This node is disabled and will not be called.\nDrag off pins to build functionality.
)

(fn ConstructionScript
  (|CallParentFunction))