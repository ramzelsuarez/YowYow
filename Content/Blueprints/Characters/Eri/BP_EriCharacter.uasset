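; Character Blueprint for Eri that hooks up the demo HUD and hurt feedback.
; BeginPlay creates WBP_HUD_DEMO with Eri's health and trick gauge components, and binds a damage event that plays a hurt sound at the character's location.
; Tick prints the action, attack, life and locomotion states from CharacterStateComponent to screen as debug text.
; Homing and attack-type debug prints are present but unconnected.
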(event Custom|OnHealthDamageTaken_Event
  (params (HealthComponent :type Health%20Component%20Object%20Reference) (Damage :type Integer) (CurrentHealth :type Integer) (DamageCauser :type Actor%20Object%20Reference) (DamageInstigator :type Controller%20Object%20Reference))
  (Audio|PlaySoundatLocation "/Game/Assets/Audio/SFX/SFX_EriHurt_Cue.SFX_EriHurt_Cue" (Transformation|GetActorLocation) "0, 0, 0" 1.0 1.0 0.0 0 0 0 0))

(event EventBeginPlay
  (Utilities|FlowControl|Sequence
    (:then_0
      (bind _returnvalue (UserInterface|CreateWidget "/Game/Blueprints/UI/WBP_HUD_DEMO.WBP_HUD_DEMO_C"))
      (UserInterface|Viewport|AddtoViewport _returnvalue 0)
      (Default|InitHUD _returnvalue (Variables|Default|GetHealthComponent) (Variables|Default|GetTrickGauge) self))
    (:then_1
      (EventDispatchers|AssignOnHealthDamageTaken (Variables|Default|GetHealthComponent) (delegate Custom|OnHealthDamageTaken_Event)))))

(event EventTick
  (params (DeltaSeconds :type Float%20%28single-precision%29))
  (bind _characterstatecomponent (Variables|Default|GetCharacterStateComponent))
  (Utilities|FlowControl|Sequence
    (:then_0
      (Development|PrintString (Utilities|String|Append "[ACTION STATE] " (Utilities|String|EnumtoString (Variables|/Script/YowYow.CharacterStateComponent|GetActionState _characterstatecomponent))) true true "(R=0.000000,G=0.660000,B=1.000000,A=1.000000)" 0.0 "1")
      (Development|PrintString (Utilities|String|Append "[ATTACK STATE] " (Utilities|String|EnumtoString (Variables|/Script/YowYow.CharacterStateComponent|GetAttackState _characterstatecomponent))) true true "(R=0.000000,G=0.660000,B=1.000000,A=1.000000)" 0.0 "2")
      (Development|PrintString (Utilities|String|Append "[LIFE STATE] " (Utilities|String|EnumtoString (Variables|/Script/YowYow.CharacterStateComponent|GetLifeState _characterstatecomponent))) true true "(R=0.000000,G=0.660000,B=1.000000,A=1.000000)" 0.0 "3")
      (Development|PrintString (Utilities|String|Append "[LOCOMOTION STATE] " (Utilities|String|EnumtoString (Variables|/Script/YowYow.CharacterStateComponent|GetLocomotionState _characterstatecomponent))) true true "(R=0.000000,G=0.660000,B=1.000000,A=1.000000)" 0.0 "4"))))

(fn ConstructionScript)