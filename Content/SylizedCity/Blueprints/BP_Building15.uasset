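; BP_Building15 is a city building Blueprint assembled from wall and block mesh components, with configurable left and right sides.
; Its Construction Script checks the Left and Right booleans, and for each enabled side hides a set of wall meshes and shows a matching set of block meshes.
; The event graph holds only disabled default events, so the Blueprint has no runtime logic.
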(event EventBeginPlay)

(event Collision|EventActorBeginOverlap
  (params (OtherActor :type Actor%20Object%20Reference)))

(event EventTick
  (params (DeltaSeconds :type Float%20%28single-precision%29)))

(fn ConstructionScript
  (if (Variables|Default|GetLeft)
    (Rendering|SetVisibility (Variables|Default|GetSM_Wall196_399) false false)
    (Rendering|SetVisibility (Variables|Default|GetSM_BlockC29) true false))
  (if (Variables|Default|GetRight)
    (Rendering|SetVisibility (Variables|Default|GetSM_Wall351) false false)
    (Rendering|SetVisibility (Variables|Default|GetSM_BlockC18) true false)))